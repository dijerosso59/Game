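; BP_Gun is a shooter weapon that fires BP_Projectile actors repeatedly from its ProjectileSpawnPoint.
; StartFiring fires one shot immediately, then runs a looping timer on FireProjectile at a rate derived from ProjectilePerSecond.
; A DoOnce gate ignores repeated start calls until StopFiring clears the timer and resets it.
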(event `FireProjectile`
  ;[1 1 1] Apparition du projectile sur le ProjectileSpawnPoint
  (`|SpawnActorFromClass` "/Game/Shooter/Core/BP_Projectile.BP_Projectile_C" (`SceneComponent.K2_GetComponentToWorld` (`self.ProjectileSpawnPoint`)) "Undefined" "OverrideRootScale" null null))

(event `StartFiring`
  ;[1 1 1] Tire des projectiles de maniere répétée
  (`/Engine/EditorBlueprintResources/StandardMacros.DoOnce` false :!label _label
    (:`Completed`
      (`self.FireProjectile`)
      (`KismetSystemLibrary.K2_SetTimer` null "FireProjectile" (/ 1.0 (`self.ProjectilePerSecond`)) true))))

(event `StopFiring`
  ;[1 1 1] Interrompt le tir de projectiles
  (`KismetSystemLibrary.K2_ClearTimer` null "FireProjectile")
  (goto _label :!via `Reset`))

(fn `UserConstructionScript`)