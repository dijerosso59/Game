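; BP_Spawner is an enemy spawner for the shooter that creates BP_Enemy AI pawns inside a box zone.
; It registers itself with the Game Mode on BeginPlay and exposes a SpawnOneEnemy event.
; That event asks the Game Mode for permission, spawns the enemy at a random point within the EnnemiesSpawnZone bounds, then tells the Game Mode to increment its enemy count.
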(event `self.ReceiveBeginPlay`
  ;[1 1 1] Envoie sa référence au Game Mode
  (message `/Game/Shooter/Core/BPI_GameModeMP.RegisterSpawner` (`GameplayStatics.GetGameMode`) self))

(event `SpawnOneEnemy`
  (bind _ennemiesspawnzone (`self.EnnemiesSpawnZone`))
  ;[0 1 0.1005] Prend une position aléatoire dans le boite et fait apparaitre un ennemie avec son IA
  (bind _bresult (message `/Game/Shooter/Core/BPI_GameModeMP.CanSpawnOneEnemy` (`GameplayStatics.GetGameMode`))) ; Demande l'autorisation de faire apparaitre\nun ennemie au Game Mode
  (if _bresult
    (`AIBlueprintHelperLibrary.SpawnAIFromClass` "/Game/Shooter/Core/BP_Enemy.BP_Enemy_C" null (`KismetMathLibrary.RandomPointInBoundingBox` (`SceneComponent.K2_GetComponentLocation` _ennemiesspawnzone) (`BoxComponent.GetScaledBoxExtent` _ennemiesspawnzone)) (struct) false null)
    (message `/Game/Shooter/Core/BPI_GameModeMP.AddOneEnemy` (`GameplayStatics.GetGameMode`)) ; Demande au Game Mode\nd'incrementer le nombre d'ennemie
  ))

(fn `UserConstructionScript`)