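; Player hero of a twin-stick shooter, with world-axis movement and a look stick that both aims and fires.
; Tilting the look stick past a dead zone sets control rotation and fires the child-actor gun; releasing stops it.
; Damage updates inherited health and the GameMode's UI; death disables input and firing.
; The AnimBP calls TriggerDeath after the death animation, so GameMode respawns the player at the transform saved on BeginPlay.
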(event `self.ReceiveBeginPlay`
  ;[1 1 1] Begin play
  (`parent.ReceiveBeginPlay`)
  (`|ExecutionSequence`
    (:`then_0`
      (bind _asbp_gun (cast `/Game/Shooter/Core/BP_Gun` (`ChildActorComponent.ChildActor` (`self.GunActor`))))
      (set `self.Gun` _asbp_gun))
    (:`then_1`
      (bind _asbp_game_mode (cast `/Game/Shooter/Core/BP_GameMode` (`GameplayStatics.GetGameMode`)))
      (bind _output_get (set `self.GameMode` _asbp_game_mode))
      (`/Game/Shooter/Core/BP_GameMode.SetPlayerSpawnTransform` _output_get (`self.GetTransform`))
      (`GameplayStatics.SpawnSoundAttached` "/Game/Shooter/Audio/A_PlayerRespawn_Cue1.A_PlayerRespawn_Cue1" (`self.CapsuleComponent`) "None" (0.0 0.0 0.0) (struct) "SnapToTarget" true 1.0 1.0 0.0 null null)
      (message `/Game/Shooter/Core/BPI_GameModeMP.UpdateUI_PlayerHealth` (`GameplayStatics.GetGameMode`) (`self.GetNormalizeHealthPoints`)))))

(event `InputAxis|MoveY`
  (params (AxisValue :type "Float (single-precision)"))
  ;[1 1 1] Déplacements
  (`self.AddMovementInput` (1.0 0.0 0.0) AxisValue))

(event `InputAxis|LookY`
  (params (AxisValue :type "Float (single-precision)"))
  (bind _gun (`self.Gun`))
  ;[1 1 1] Orientation
  (bind _returnvalue (`KismetMathLibrary.MakeVector` AxisValue (stale `InputAxis|LookX` AxisValue)))
  (if (> (`KismetMathLibrary.VSize` _returnvalue) 0.25) :!label _label
    (`Controller.SetControlRotation` (`GameplayStatics.GetPlayerController` 0) (`KismetMathLibrary.Conv_VectorToRotator` _returnvalue))
    ;[1 1 1] Tir des projectiles lorqu'on incline le stick et arrête de tirer lorsqu'on n'incline plus le stick
    (`/Game/Shooter/Core/BP_Gun.StartFiring` _gun)
    (else
      (`/Game/Shooter/Core/BP_Gun.StopFiring` _gun))))

(event `InputAxis|LookX`
  (params (AxisValue :type "Float (single-precision)"))
  ;[1 1 1] Orientation
  (goto _label))

(event `InputAxis|MoveX`
  (params (AxisValue :type "Float (single-precision)"))
  ;[1 1 1] Déplacements
  (`self.AddMovementInput` (0.0 1.0 0.0) AxisValue))

(event `/Game/Shooter/Core/BPI_Damageable.AffectHealth`
  (params (Delta :type "Float (single-precision)"))
  ;[1 1 1] Gestion des points de vie du héros
  (if (not (`self.Mort`))
    (`self.UpdateVie` Delta)
    (message `/Game/Shooter/Core/BPI_GameModeMP.UpdateUI_PlayerHealth` (`GameplayStatics.GetGameMode`) (`self.GetNormalizeHealthPoints`))
    (`GameplayStatics.SpawnSoundAttached` "/Game/Shooter/Audio/Hit_Cue.Hit_Cue" (`self.CapsuleComponent`) "None" (0.0 0.0 0.0) (struct) "KeepRelativeOffset" false 1.0 1.0 0.0 null null)
    (if (`self.Mort`)
      (`self.DisableInput` (`GameplayStatics.GetPlayerController` 0))
      (`/Game/Shooter/Core/BP_Gun.StopFiring` (`self.Gun`))
      (`GameplayStatics.SpawnSoundAtLocation` "/Game/Shooter/Audio/A_PlayerDeath_Cue.A_PlayerDeath_Cue" (`self.K2_GetActorLocation`) (struct) 1.0 1.0 0.0 null null))))

(event `self.TriggerDeath`
  ;[1 1 1] Event appelé par l'ABP lorsqu'il a finit de jouer l'animation de mort du joueur
  (`parent.TriggerDeath`)
  (if (`self.Mort`)
    (`/Game/Shooter/Core/BP_GameMode.RespawnPlayer` (`self.GameMode`))
    (`self.K2_DestroyActor`)))

(fn `UserConstructionScript`
  (`parent.UserConstructionScript`))