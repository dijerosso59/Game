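; Shooter game mode that handles hero respawning and tracks the enemy population against a cap.
; RespawnPlayer spawns a BP_hero at the stored start transform and has player controller 0 possess it.
; RegisterSpawner stores the map's spawner and starts a looping timer at the enemy spawn rate.
; Counter events and a capacity check manage the enemy count, which Tick prints on screen each frame.
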(event `RespawnPlayer`
  ;[1 1 1] Fais réapparaitre le héros dans le monde et branche le controller du player sur lui
  (bind _returnvalue (`|SpawnActorFromClass` "/Game/Shooter/Core/BP_hero.BP_hero_C" (`self.PlayerSpawnTransform`) "Undefined" "OverrideRootScale" null null))
  (`Controller.Possess` (`GameplayStatics.GetPlayerController` 0) _returnvalue) ; Dire au controller du player de prendre\npossession du pawn
)

(event `self.ReceiveTick`
  (params (DeltaSeconds :type "Float (single-precision)"))
  (`KismetSystemLibrary.PrintString` (`KismetStringLibrary.Concat_StrStr` "Nombre d'ennemis =" (`KismetStringLibrary.Conv_IntToString` (`self.CurrentEnemyCount`))) true true (struct :`R` 1.0 :`G` 0.892962 :`A` 1.0) 0.0))

(event `/Game/Shooter/Core/BPI_GameModeMP.RegisterSpawner`
  (params (NewSpawner :type "/Game/Shooter/Core/BP_Spawner Object Reference"))
  ;[1 1 1] Récupère une référence vers le spawner de la map et lance le spawn des ennemis
  (set `self.Spawner` NewSpawner)
  (`KismetSystemLibrary.K2_SetTimerDelegate` (`|CreateDelegate` (`self.Spawner`) :!event `SpawnOneEnemy`) (/ 1.0 (`self.EnemiersPerSecond`)) true))

(event `/Game/Shooter/Core/BPI_GameModeMP.AddOneEnemy`
  ;[1 1 1] Gère le nombre d'ennemie sur la map
  (`/Engine/EditorBlueprintResources/StandardMacros.IncrementInt` (`self.CurrentEnemyCount`)))

(event `/Game/Shooter/Core/BPI_GameModeMP.RemoveOneEnemy`
  ;[1 1 1] Gère le nombre d'ennemie sur la map
  (`/Engine/EditorBlueprintResources/StandardMacros.DecrementInt` (`self.CurrentEnemyCount`)))

(fn `CanSpawnOneEnemy`
  (returns (bResult :type Boolean))
  (return (< (`self.CurrentEnemyCount`) (`self.MaxEnemyCount`))))

(fn `GetEnnemyCount`
  (returns (Count :type Integer))
  (return (`self.CurrentEnemyCount`)))

(fn `SetPlayerSpawnTransform`
  (params (PlayerSpawnTransform :type "Transform Structure"))
  ;[1 1 1] Stock la position de départ du joueur
  (set `self.PlayerSpawnTransform` PlayerSpawnTransform)
  (return))

(fn `UserConstructionScript`)