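; BP_Character is a character Blueprint for the shooter that tracks health (Vie) and death state (Mort).
; UpdateVie adds a signed difference to Vie without clamping, calls UpdateMort and returns the new value.
; The UpdateMort event sets Mort true when Vie is zero or below, and false otherwise.
; BeginPlay, overlap, Tick and the construction script are empty.
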(event `UpdateMort`
  ;[1 1 1] Vérifie si le personnage n'as plus de points de vie
  (if (<= (`self.Vie`) 0.0)
    (set `self.Mort` true)
    (else
      (set `self.Mort` false))))

(fn `UpdateVie`
  (params (Difference :type "Float (double-precision)"))
  (returns (NewVie :type "Float (double-precision)"))
  ;[1 1 1] Mise à jour des points de vie
  (bind _output_get (set `self.Vie` (+ Difference (`self.Vie`))))
  (`self.UpdateMort`)
  (return _output_get))

(fn `UserConstructionScript`)