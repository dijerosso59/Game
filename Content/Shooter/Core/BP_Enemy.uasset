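; BP_Enemy is a shooter enemy that hurts the hero on contact and can be killed.
; Overlapping PlayerDamageBox damages BP_hero immediately, then on a looping timer paced by AttacksPerSecond until the hero leaves.
; AffectHealth updates health and, on death (Mort), detaches the controller, disables capsule collision and plays a death sound.
; TriggerDeath, called when the animation Blueprint finishes the death animation, notifies the game mode and destroys the actor.
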(event `/Game/Shooter/Core/BPI_Damageable.AffectHealth`
  (params (Delta :type "Float (single-precision)"))
  ;[1 1 1] Gestion des dégats
  (if (not (`self.Mort`))
    (bind _newvie (`self.UpdateVie` Delta))
    (`KismetSystemLibrary.PrintString` (`KismetStringLibrary.Conv_DoubleToString` _newvie))
    (if (`self.Mort`)
      (`self.DetachFromControllerPendingDestroy`)
      (`PrimitiveComponent.SetCollisionEnabled` (`self.CapsuleComponent`) "NoCollision")
      (`GameplayStatics.SpawnSoundAttached` "/Game/Shooter/Audio/A_EnemyDeath_Cue.A_EnemyDeath_Cue" (`self.CapsuleComponent`) "None" (0.0 0.0 0.0) (struct) "SnapToTarget" false 1.0 1.0 0.0 null null))))

(event `self.TriggerDeath`
  ;[1 1 1] Event appelé lorsque l'ABP a fini de jouer l'animation de mort
  (`parent.TriggerDeath`)
  (message `/Game/Shooter/Core/BPI_GameModeMP.RemoveOneEnemy` (`GameplayStatics.GetGameMode`))
  (`self.K2_DestroyActor`))

(event `self.PlayerDamageBox.OnComponentBeginOverlap`
  (params (OverlappedComponent :type "PrimitiveComponent Object Reference") (OtherActor :type "Actor Object Reference") (OtherComp :type "PrimitiveComponent Object Reference") (OtherBodyIndex :type Integer) (bFromSweep :type Boolean) (SweepResult :type "HitResult Structure (by ref)"))
  ;[1 1 1] Commence à faire des dégats au héros à intervalles réguliers
  (bind _asbp_hero (cast `/Game/Shooter/Core/BP_hero` OtherActor))
  (set `self.Hero` _asbp_hero)
  (`self.DamageHero`)
  (bind _returnvalue (`KismetSystemLibrary.K2_SetTimerDelegate` (`|CreateDelegate` :!event `DamageHero`) (/ 1.0 (`self.AttacksPerSecond`)) true))
  (set `self.Timer` _returnvalue))

(event `DamageHero`
  ;[1 1 1] Commence à faire des dégats au héros à intervalles réguliers
  ;;[1 1 1] Arrête de faire des dégats au héros
  ;;;[1 1 1] Fait des dégats au héros une fois
  (`/Game/Shooter/Core/BP_hero.AffectHealth` (`self.Hero`) (`self.DamageAmmount`)))

(event `self.PlayerDamageBox.OnComponentEndOverlap`
  (params (OverlappedComponent :type "PrimitiveComponent Object Reference") (OtherActor :type "Actor Object Reference") (OtherComp :type "PrimitiveComponent Object Reference") (OtherBodyIndex :type Integer))
  ;[1 1 1] Commence à faire des dégats au héros à intervalles réguliers
  ;;[1 1 1] Arrête de faire des dégats au héros
  ;;;[1 1 1] Fait des dégats au héros une fois
  (if (== OtherActor (`self.Hero`))
    (`KismetSystemLibrary.K2_ClearAndInvalidateTimerHandle` (`self.Timer`))))

(fn `UserConstructionScript`
  (`parent.UserConstructionScript`))